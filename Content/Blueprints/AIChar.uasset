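; AI-controlled armed character that takes cover, shoots and ragdolls on death before being destroyed after a delay.
; Threats switch it to the EnemyShootCover behavior tree and set its focal point; leaving cover uncrouches and runs AI_BTree.
; The construction script caches the socketed child-actor weapon as CurrentGun, which handles start/stop shooting; ShootEnemy only spawns muzzle FX.
; Damage reduces Health, playing a react montage until death stops AI logic and shooting.
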(event Custom|StartShooting
  (Default|StartShooting (Variables|Default|GetCurrentGun)))

(event Custom|StopShooting
  (Default|StopShooting (Variables|Default|GetCurrentGun)))

(event Custom|GetOutOfCover
  (Variables|Default|SetIsInCover false)
  (Character|UnCrouch)
  (bind _asaicontrol (Utilities|Casting|CastToAIControl (AI|GetAIController self)))
  (AI|RunBehaviorTree _asaicontrol "/Game/Blueprints/AI/AI_BTree.AI_BTree"))

(event Custom|ShootEnemy
  (params (Enemy :type Actor%20Object%20Reference))
  (CallFunction|PlayShootFX))

(event Custom|Play%20Shoot%20FX
  (bind _weapon (Variables|Default|GetWeapon))
  (Effects|SpawnEmitteratLocation 0 (Transformation|GetSocketLocation _weapon "Socket") (Transformation|GetSocketRotation _weapon "Socket")))

(event Custom|Threatened
  (params (ThreatSource :type Vector))
  (bind _self self)
  (bind _returnvalue (AI|GetAIController _self))
  (AI|RunBehaviorTree _returnvalue "/Game/Blueprints/AI/EnemyShootCover.EnemyShootCover")
  (AI|SetFocalPoint _returnvalue ThreatSource))

(event Custom|EnterCover
  (Variables|Default|SetIsInCover true)
  (Character|Crouch)
  (Utilities|Casting|CastToAIControl (AI|GetAIController self)))

(event EventBeginPlay
  (AI|Components|Blackboard|SetValueasBool (AI|GetBlackboard 0) (Utilities|Name|MakeLiteralName "Static") (Variables|Default|GetStatic)))

(event Game|Damage|EventAnyDamage
  (params (Damage :type Float%20%28single-precision%29) (DamageType :type Damage%20Type%20Object%20Reference) (InstigatedBy :type Controller%20Object%20Reference) (DamageCauser :type Actor%20Object%20Reference))
  (bind _output_get (Variables|Default|SetHealth (- (Variables|Default|GetHealth) Damage)))
  (if (<= _output_get 0.0)
    (Physics|SetSimulatePhysics (Variables|Character|GetMesh) true)
    (AI|Logic|StopLogic (Variables|/Script/AIModule.AIController|GetBrainComponent (AI|GetAIController self)) "")
    (Collision|SetCollisionEnabled (Variables|Collision|GetCapsuleComponent) "NoCollision")
    (Collision|SetCollisionResponsetoChannel (Variables|Character|GetMesh) "ECC_Pawn" "ECR_Ignore")
    (CallFunction|StopShooting)
    (Utilities|FlowControl|Delay 2e+01)
    (Actor|DestroyActor)
    (else
      (Animation|Montage|PlayMontage (Variables|Character|GetMesh) "/Game/AnimStarterPack/React_Montage.React_Montage"))))

(fn ConstructionScript
  (Transformation|AttachComponentToComponent (Variables|Default|GetWeapon) (Variables|Character|GetMesh) "WeaponSocket" "SnapToTarget" "SnapToTarget" "SnapToTarget" true)
  (bind _asweapon (Utilities|Casting|CastToWeapon (Variables|/Script/Engine.ChildActorComponent|GetChildActor (Variables|Default|GetWeapon))))
  (Variables|Default|SetCurrentGun _asweapon))