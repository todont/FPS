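; EncounterSpace is a Blueprint volume that shares a target location with the AI characters inside it.
; Its CallOutTarget event stores the given location, then loops over every AIChar actor and keeps those overlapping the space.
; For each of those, it writes the location to the MoveLocation blackboard key and sets CanSeePlayer to true, so one call-out alerts the whole group.
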(event Custom|CallOutTarget
  (params (TargetLocation :type Vector))
  (Variables|Default|SetTargetLocation TargetLocation)
  (bind _outactors (Actor|GetAllActorsOfClass "/Game/Blueprints/AIChar.AIChar_C"))
  (for _array_element _outactors
    (if (Collision|IsOverlappingActor _array_element :!class /Script/Engine.Actor)
      (AI|Components|Blackboard|SetValueasVector (AI|GetBlackboard _array_element) (Utilities|Name|MakeLiteralName "MoveLocation") (Variables|Default|GetTargetLocation))
      (AI|Components|Blackboard|SetValueasBool (AI|GetBlackboard _array_element) (Utilities|Name|MakeLiteralName "CanSeePlayer") true))))

(fn ConstructionScript)