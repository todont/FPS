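; Behavior tree task that makes an AI character start shooting, and stop shooting when the task is aborted.
; On execute it checks whether the blackboard cover location is within range while the character is not already in cover, printing the distance for debugging.
; If so, it switches the controller to the EnemyShootCover behavior tree.
; The task never calls finish execute, so it keeps running until aborted or replaced.
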(event EventReceiveExecuteAI
  (params (OwnerController :type AI%20Controller%20Object%20Reference) (ControlledPawn :type Pawn%20Object%20Reference))
  (bind _output_get (Variables|Default|SetPawn ControlledPawn))
  (bind _asaichar (Utilities|Casting|CastToAIChar _output_get))
  (Default|StartShooting _asaichar)
  (bind _iscoverclose (CallFunction|IsCoverClose))
  (if _iscoverclose
    (AI|RunBehaviorTree OwnerController "/Game/Blueprints/AI/EnemyShootCover.EnemyShootCover")))

(event EventReceiveAbortAI
  (params (OwnerController :type AI%20Controller%20Object%20Reference) (ControlledPawn :type Pawn%20Object%20Reference))
  (bind _asaichar (Utilities|Casting|CastToAIChar ControlledPawn))
  (Default|StopShooting _asaichar)
  (Class|BTTaskBlueprintBase|FinishAbort))

(fn IsCoverClose
  (bind _pawn (Variables|Default|GetPawn))
  (bind _bb_coverlocation (Variables|Default|GetBB_CoverLocation))
  (bind _returnvalue (Transformation|GetActorLocation _pawn))
  (bind _returnvalue_2 (Class|BTFunctionLibrary|GetBlackboardValueasVector _bb_coverlocation))
  (bind _returnvalue_3 (Math|Vector|Distance(Vector) _returnvalue_2 _returnvalue))
  (Development|PrintString (Utilities|String|ToString(Float) _returnvalue_3))
  (return (and (< _returnvalue_3 1e+03) (not (Class|BTFunctionLibrary|GetBlackboardValueasBool (Variables|Default|GetBB_IsInCover))))))