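; Behavior tree task that moves an AI pawn to a cover location and puts it into cover.
; It runs AI MoveTo toward the BBMove blackboard vector, then calls EnterCover on the pawn as either an Enemy or an AIChar.
; It then sets the BBInCover flag and finishes successfully; a pawn of neither class leaves the task unfinished.
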(event EventReceiveExecuteAI
  (params (OwnerController :type AI%20Controller%20Object%20Reference) (ControlledPawn :type Pawn%20Object%20Reference))
  (AI|AIMoveTo OwnerController (Class|BTFunctionLibrary|GetBlackboardValueasVector (Variables|Default|GetBB_Move)) 0 -1.0 "Default" "Default" true true
    (:OnMoveFinished
      (bind _asenemy (Utilities|Casting|CastToEnemy ControlledPawn)
        (:then
          (Default|EnterCover _asenemy)
          (Class|BTFunctionLibrary|SetBlackboardValueasBool (Variables|Default|GetBB_InCover) true)
          (AI|BehaviorTree|FinishExecute true))
        (:CastFailed
          (bind _asaichar (Utilities|Casting|CastToAIChar ControlledPawn))
          (Default|EnterCover _asaichar)
          (Class|BTFunctionLibrary|SetBlackboardValueasBool (Variables|Default|GetBB_InCover) true)
          (AI|BehaviorTree|FinishExecute true))))))