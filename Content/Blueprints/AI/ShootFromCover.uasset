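; Behavior tree task that makes an AIChar stand up from cover, shoot, then duck back down.
; On execute it uncrouches the pawn and starts shooting, and a three-second timer then stops the fire, crouches the pawn and finishes successfully.
; Each tick sets the controller's focal point to player 0's location.
; Abort stops shooting and leaves the pawn standing.
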(event Custom|StopShooting
  (Default|StopShooting (Variables|Default|GetPawn))
  (Character|Crouch (Variables|Default|GetPawn))
  (AI|BehaviorTree|FinishExecute true))

(event EventReceiveExecuteAI
  (params (OwnerController :type AI%20Controller%20Object%20Reference) (ControlledPawn :type Pawn%20Object%20Reference))
  (bind _asaichar (Utilities|Casting|CastToAIChar ControlledPawn))
  (bind _output_get (Variables|Default|SetPawn _asaichar))
  (Character|UnCrouch _output_get)
  (Default|StartShooting (Variables|Default|GetPawn))
  (Utilities|Time|SetTimerbyEvent (delegate Custom|StopShooting) 3.0))

(event EventReceiveTickAI
  (params (OwnerController :type AI%20Controller%20Object%20Reference) (ControlledPawn :type Pawn%20Object%20Reference) (DeltaSeconds :type Float%20%28single-precision%29))
  (AI|SetFocalPoint OwnerController (Transformation|GetActorLocation (Game|GetPlayerCharacter 0))))

(event EventReceiveAbortAI
  (params (OwnerController :type AI%20Controller%20Object%20Reference) (ControlledPawn :type Pawn%20Object%20Reference))
  (bind _pawn (Variables|Default|GetPawn))
  (Character|UnCrouch _pawn)
  (Default|StopShooting _pawn)
  (Class|BTTaskBlueprintBase|FinishAbort))