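; Enemy character that carries a gun, can fire it and can crouch into cover.
; The construction script snaps the Weapon child actor component to the mesh's Weapon socket, and BeginPlay casts its spawned actor to Weapon and stores it as CurrentGun.
; StartShooting and StopShooting forward to that gun, while EnterCover sets IsInCover and crouches.
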(event OnComponentHit(CapsuleComponent)
  (params (HitComponent :type Primitive%20Component%20Object%20Reference) (OtherActor :type Actor%20Object%20Reference) (OtherComp :type Primitive%20Component%20Object%20Reference) (NormalImpulse :type Vector :default "0, 0, 0") (Hit :type Hit%20Result%20Structure%20%28by%20ref%29)))

(event Custom|StartShooting
  (Default|StartShooting (Variables|Default|GetCurrentGun)))

(event Custom|StopShooting
  (Default|StopShooting (Variables|Default|GetCurrentGun)))

(event Custom|EnterCover
  (Variables|Default|SetIsInCover true)
  (Character|Crouch))

(event EventBeginPlay
  (bind _asweapon (Utilities|Casting|CastToWeapon (Variables|/Script/Engine.ChildActorComponent|GetChildActor (Variables|Default|GetWeapon))))
  (Variables|Default|SetCurrentGun _asweapon))

(fn ConstructionScript
  (Transformation|AttachComponentToComponent (Variables|Default|GetWeapon) (Variables|Character|GetMesh) "Weapon" "SnapToTarget" "SnapToTarget" "SnapToTarget" true))