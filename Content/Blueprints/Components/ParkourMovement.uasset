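; Parkour movement component that adds wall running, vertical wall running, ledge grabs, mantling and wall jumps to a Character.
; A 60 Hz looping timer drives gated macros that trace for surfaces, then launch or interpolate the character and tilt the camera.
; Movement-mode, jump and landing events toggle the gates, while a parkour-type state arbitrates moves and restores gravity and movement mode.
; Sprint is partly wired, while crouch and slide functions are empty stubs.
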(event Custom|Initialize
  (params (Character :type Character%20Object%20Reference))
  (bind _output_get (Variables|Default|SetCharacter Character))
  (bind _output_get_2 (Variables|Default|SetCharacter_Movement (Variables|/Script/Engine.Character|GetCharacterMovement _output_get)))
  (Variables|Default|SetDefaultGravity (Variables|/Script/Engine.CharacterMovementComponent|GetGravityScale _output_get_2))
  (Utilities|Time|SetTimerbyEvent (delegate Custom|WallRunUpdate) 0.0167 true))

(event Custom|Land_Event
  (CallFunction|WallRunEnd 0.0)
  (CallFunction|VerticalWallRunEnd 0.0)
  (CallFunction|CloseGates)
  (CallFunction|PlayCameraShake "/Game/Blueprints/Components/CameraShakes/JumpLand.JumpLand_C"))

(event Custom|Jump_Event
  (if (Utilities|Enum|Equal(Enum) (Variables|Default|GetCurrentParkourType) "NewEnumerator0")
    (if (not (AI|Components|NavMovement|IsFalling (Variables|Default|GetCharacter_Movement)))
      (CallFunction|OpenGates))
    (else
      (CallFunction|JumpEvents))))

(event Custom|WallRunUpdate
  (Utilities|FlowControl|Sequence
    (:then_0
      (|WallRun))
    (:then_1
      (|VerticalWallRun))
    (:then_2
      (|Mantle))
    (:then_3
      (CallFunction|CameraTick))))

(event Custom|ResetWallRunSuppression)

(event Custom|ParkourMovementChange
  (params (PrevParkourType :type EParkourMovementType%20Enum :default "NewEnumerator0") (NewParkourType :type EParkourMovementType%20Enum :default "NewEnumerator0"))
  (Variables|Default|SetPrevParkourType PrevParkourType)
  (Variables|Default|SetCurrentParkourType NewParkourType)
  (CallFunction|ResetMovement))

(event Custom|MovementChange
  (params (PrevMovementMode :type EMovementMode%20Enum :default "MOVE_None") (NewMovementMode :type EMovementMode%20Enum :default "MOVE_None"))
  (Utilities|IsValid (Variables|Default|GetCharacter_Movement)
    (:Is%20Valid
      (Variables|Default|SetPrevMovement%20Mode PrevMovementMode)
      (Variables|Default|SetCurrentMovementMode NewMovementMode)
      (|OpenGatesNode))))

(event Custom|SprintEvent
  (CallFunction|SprintStart))

(event Custom|CrouchSlideEvent
  (|ParkourCancel
    (:Clear
      (if (Utilities|CanSlide)
        _))))

(event Custom|PlayCameraShake
  (params (Shake :type Matinee%20Camera%20Shake%20Class%20Reference))
  (if (Variables|Default|GetCameraShake)
    (Camera|PlayWorldCameraShake Shake (Transformation|GetActorLocation (Variables|Default|GetCharacter)) 0.0 1e+02)))

(event EventBeginPlay)

(fn WallRunReset
  (if (Utilities|CanWallRun)
    (bind _onwall (CallFunction|WallRunMovement (Transformation|GetActorLocation (Variables|Default|GetCharacter)) (.RightEndPoint (Utilities|WallRunEndVectors)) -1.0))
    (if _onwall
      (CallFunction|SetParkourType "NewEnumerator2")
      (Variables|/Script/Engine.CharacterMovementComponent|SetGravityScale (Variables|Default|GetCharacter_Movement) (Math|Interpolation|FInterpTo (Variables|/Script/Engine.CharacterMovementComponent|GetGravityScale (Variables|Default|GetCharacter_Movement)) (Variables|Default|GetWallRunTargetGravity) (Utilities|Time|GetWorldDeltaSeconds) 1e+01) :!label _label)
      (elif (Utilities|Enum|Equal(Enum) (Variables|Default|GetCurrentParkourType) "NewEnumerator2")
        (CallFunction|WallRunEnd 0.5)
        (else
          (bind _onwall_2 (CallFunction|WallRunMovement (Transformation|GetActorLocation (Variables|Default|GetCharacter)) (.LeftEndPoint (Utilities|WallRunEndVectors)) 1.0))
          (if _onwall_2
            (CallFunction|SetParkourType "NewEnumerator1")
            (goto _label)
            (else
              (CallFunction|WallRunEnd 0.5))))))
    (else
      (CallFunction|WallRunEnd 0.0))))

(fn WallRunMovement
  (params (Start :type Vector) (End :type Vector) (Direction :type Float%20%28single-precision%29))
  (bind _outhit (Collision|LineTraceByChannel Start End "TraceTypeQuery1" false 0 "None"))
  (if (.bblockinghit _outhit)
    (if (and (AI|Components|NavMovement|IsFalling (Variables|Default|GetCharacter_Movement)) (.ReturnValue (Utilities|ValidWallRunVector (.normal _outhit))))
      (Variables|Default|SetWallRunNormal (.OutVec (Utilities|ValidWallRunVector (.normal _outhit))))
      (Character|LaunchCharacter (Variables|Default|GetCharacter) (* (Math|Vector|CrossProduct (Variables|Default|GetWallRunNormal) "0, 0,1.000000") (* (Variables|Default|GetWallRunSpeed) Direction)) false (not (Variables|Default|GetWallRunGravity))) ; Run Forward
      (return true)
      (else
        (return false)))
    (else
      (return false))))

(fn WallRunEnd
  (params (ResetTime :type Float%20%28single-precision%29))
  (if (Utilities|IsWallRunning)
    (bind _changed (CallFunction|SetParkourType "NewEnumerator0"))
    (if _changed
      (CallFunction|CloseWallRunGate)
      (Utilities|Time|SetTimerbyFunctionName 0 "OpenWallRunGate" ResetTime))))

(fn CameraTick
  (switch Utilities|FlowControl|Switch|SwitchonEParkourMovementType (Variables|Default|GetCurrentParkourType)
    (:NewEnumerator0
      (CallFunction|CameraTilt 0.0 :!label _label))
    (:NewEnumerator1
      (CallFunction|CameraTilt 15.0))
    (:NewEnumerator2
      (CallFunction|CameraTilt -15.0))
    (:NewEnumerator3
      (goto _label))
    (:NewEnumerator4
      (goto _label))
    (:NewEnumerator5
      (goto _label))
    (:NewEnumerator6
      (CallFunction|CameraTilt -8.0))
    (:NewEnumerator7
      (goto _label))))

(fn CameraTilt
  (params (Xroll :type Float%20%28single-precision%29))
  (bind _character (Variables|Default|GetCharacter))
  (bind _returnvalue (Pawn|GetController _character))
  (bind _returnvalue_2 (Pawn|GetControlRotation _returnvalue :!class /Script/Engine.Controller))
  (bind (_roll _pitch _yaw) (Math|Rotator|BreakRotator _returnvalue_2))
  (Pawn|SetControlRotation (Pawn|GetController (Variables|Default|GetCharacter)) (Math|Interpolation|RInterpTo _returnvalue_2 (Math|Rotator|MakeRotator Xroll _pitch _yaw) (Utilities|Time|GetWorldDeltaSeconds) 2e+01)))

(fn WallRunJump
  (bind _wallrunnormal (Variables|Default|GetWallRunNormal))
  (bind _wallrunjumpoffforce (Variables|Default|GetWallRunJumpOffForce))
  (if (Utilities|IsWallRunning)
    (CallFunction|WallRunEnd 0.35)
    (Character|LaunchCharacter (Variables|Default|GetCharacter) (Math|Vector|MakeVector (* (.x _wallrunnormal) _wallrunjumpoffforce) (* (.y _wallrunnormal) _wallrunjumpoffforce) (Variables|Default|GetWallRunJumpHeight)) false true)))

(fn ResetMovement
  (if (Utilities|Enum|Equal(Enum) (Variables|Default|GetCurrentParkourType) "NewEnumerator0")
    (Variables|/Script/Engine.CharacterMovementComponent|SetGravityScale (Variables|Default|GetCharacter_Movement) (Variables|Default|GetDefaultGravity))
    (Pawn|Components|CharacterMovement|SetMovementMode (Variables|Default|GetCharacter_Movement) (Utilities|Select :Index (Variables|Default|GetPrevParkourType) :NewEnumerator0 "MOVE_Falling" :NewEnumerator1 "MOVE_Falling" :NewEnumerator2 "MOVE_Falling" :NewEnumerator3 "MOVE_Falling" :NewEnumerator4 "MOVE_Falling" :NewEnumerator5 "MOVE_Walking" :NewEnumerator6 "MOVE_Walking" :NewEnumerator7 "MOVE_Walking" :NewEnumerator8 "MOVE_None") 0)))

(fn SetParkourType
  (params (NewType :type EParkourMovementType%20Enum :default "NewEnumerator0"))
  (if (Utilities|Enum|Equal(Enum) NewType (Variables|Default|GetCurrentParkourType))
    (return false)
    (else
      (CallFunction|ParkourMovementChange (Variables|Default|GetCurrentParkourType) NewType)
      (return true))))

(fn VerticalWallRunUpdate
  (bind (_eyes _feet) (Utilities|MantleVectors))
  (if (Utilities|CanVerticalWallRun)
    (bind (_outhit _returnvalue) (Collision|CapsuleTraceByChannel _eyes _feet 2e+01 1e+01 "TraceTypeQuery1" false 0 "None"))
    (if _returnvalue
      (Variables|Default|SetMantleDistance (.Distance (Collision|BreakHitResult _outhit)))
      (if (Class|CharacterMovementComponent|IsWalkable (Variables|Default|GetCharacter_Movement) _outhit)
        (Variables|Default|SetMantlePosition (+ (.ImpactPoint (Collision|BreakHitResult _outhit)) (Math|Vector|MakeVector 0.0 0.0 (Variables|/Script/Engine.CapsuleComponent|GetCapsuleHalfHeight (Variables|/Script/Engine.Character|GetCapsuleComponent (Variables|Default|GetCharacter))))))
        (CallFunction|CloseVerticalWallRunGate)
        (|LedgeGrab)
        (if (Utilities|QuickMantle)
          (CallFunction|OpenMantleGateCheck)
          (else
            (Utilities|Time|SetTimerbyFunctionName 0 "OpenMantleGateCheck" 0.25)))
        (else
          (CallFunction|VerticalWallRunMovement :!label _label)))
      (else
        (goto _label)))
    (else
      (CallFunction|VerticalWallRunEnd 0.35))))

(fn VerticalWallRunEnd
  (params (ResetTime :type Float%20%28single-precision%29))
  (bind _currentparkourtype (Variables|Default|GetCurrentParkourType))
  (if (Math|Boolean|ORBoolean (Utilities|Enum|Equal(Enum) _currentparkourtype "NewEnumerator4") (Utilities|Enum|Equal(Enum) _currentparkourtype "NewEnumerator3") (Utilities|Enum|Equal(Enum) _currentparkourtype "NewEnumerator5"))
    (bind _changed (CallFunction|SetParkourType "NewEnumerator0"))
    (if _changed
      (CallFunction|CloseVerticalWallRunGate)
      (CallFunction|CloseMantleGateCheck)
      (Utilities|Time|SetTimerbyFunctionName 0 "OpenVerticalWallRunGate" ResetTime))))

(fn VerticalWallRunMovement
  (bind _feet (Utilities|MantleVectors))
  (bind (_outhit _returnvalue) (Collision|LineTraceByChannel _feet (+ (* (Transformation|GetActorForwardVector (Variables|Default|GetCharacter)) 5e+01) _feet) "TraceTypeQuery1" false 0 "None"))
  (if (and (> (Utilities|ForwardInput) 0.0) _returnvalue)
    (Variables|Default|SetVerticalWallRunNormal (.ImpactNormal (Collision|BreakHitResult _outhit)))
    (CallFunction|SetParkourType "NewEnumerator3")
    (Character|LaunchCharacter (Variables|Default|GetCharacter) (Math|Vector|MakeVector (.x (* (Variables|Default|GetVerticalWallRunNormal) -6e+02)) (.y (* (Variables|Default|GetVerticalWallRunNormal) -6e+02)) (Variables|Default|GetVerticalWallRunSpeed)) true true)
    (else
      (CallFunction|VerticalWallRunEnd 0.35))))

(fn MantleMovement
  (bind _character (Variables|Default|GetCharacter))
  (bind _mantleposition (Variables|Default|GetMantlePosition))
  (bind _character_2 (Variables|Default|GetCharacter))
  (bind _returnvalue (Pawn|GetController _character_2))
  (bind _returnvalue_2 (Transformation|GetActorLocation _character))
  (Pawn|SetControlRotation _returnvalue (Math|Interpolation|RInterpTo (Pawn|GetControlRotation _returnvalue :!class /Script/Engine.Controller) (Math|Rotator|FindLookatRotation (Math|Vector|MakeVector (.x _returnvalue_2) (.y _returnvalue_2) 0.0) (Math|Vector|MakeVector (.x _mantleposition) (.y _mantleposition) 0.0)) (Utilities|Time|GetWorldDeltaSeconds) 7.0))
  (Transformation|SetActorLocation (Variables|Default|GetCharacter) (Math|Interpolation|VInterpTo (Transformation|GetActorLocation (Variables|Default|GetCharacter)) (Variables|Default|GetMantlePosition) (Utilities|Time|GetWorldDeltaSeconds) (select (Utilities|QuickMantle) (Variables|Default|GetQuickMantleSpeed) (Variables|Default|GetDefaultMantleSpeed))) false false)
  (if (< (Math|Vector|Distance(Vector) (Transformation|GetActorLocation (Variables|Default|GetCharacter)) (Variables|Default|GetMantlePosition)) 8.0)
    (CallFunction|VerticalWallRunEnd 0.5)))

(fn OpenGates
  (CallFunction|OpenWallRunGate)
  (CallFunction|OpenVerticalWallRunGate))

(fn CloseGates
  (CallFunction|CloseWallRunGate)
  (CallFunction|CloseVerticalWallRunGate))

(fn LedgeGrabJump
  (bind _currentparkourtype (Variables|Default|GetCurrentParkourType))
  (bind _ledgegrabjumpforce (Variables|Default|GetLedgeGrabJumpForce))
  (bind _verticalwallrunnormal (Variables|Default|GetVerticalWallRunNormal))
  (if (Math|Boolean|ORBoolean (Utilities|Enum|Equal(Enum) _currentparkourtype "NewEnumerator3") (Utilities|Enum|Equal(Enum) _currentparkourtype "NewEnumerator4") (Utilities|Enum|Equal(Enum) _currentparkourtype "NewEnumerator5"))
    (CallFunction|VerticalWallRunEnd 0.0)
    (Character|LaunchCharacter (Variables|Default|GetCharacter) (Math|Vector|MakeVector (* (.x _verticalwallrunnormal) _ledgegrabjumpforce) (* (.y _verticalwallrunnormal) _ledgegrabjumpforce) (Variables|Default|GetLedgeGrabHeight)) false true)))

(fn JumpEvents
  (CallFunction|WallRunJump)
  (CallFunction|LedgeGrabJump))

(fn SprintEnd
  (if (Utilities|Enum|Equal(Enum) (Variables|Default|GetCurrentParkourType) "NewEnumerator0")
    (bind _changed (CallFunction|SetParkourType "NewEnumerator0"))
    (if _changed
      (CallFunction|CloseSprintGate)
      (Utilities|Time|SetTimerbyFunctionName 0 "OpenSprintGate" 0.1))))

(fn SprintStart
  (CallFunction|CrouchEnd)
  (CallFunction|SlideEnd)
  (if (Utilities|CanSprint)
    (CallFunction|SetParkourType "NewEnumerator7")
    (if true
      (Variables|/Script/Engine.CharacterMovementComponent|SetMaxWalkSpeed (Variables|Default|GetCharacter_Movement) (Variables|Default|GetSprintSpeed))
      (CallFunction|OpenSprintGate))))

(fn CrouchStart)

(fn CrouchEnd)

(fn SlideStart)

(fn SlideEnd)

(fn SprintUpdate
  (if (Utilities|Enum|Equal(Enum) (Variables|Default|GetCurrentParkourType) "NewEnumerator0")
    (if (> (Utilities|ForwardInput) 0.0)
      (CallFunction|SprintEnd))))

(event Custom|CloseVerticalWallRunGate
  (CallFunction|CloseMantleGate)
  (Utilities|FlowControl|Gate true) ; enters at Close
)

(event Custom|OpenVerticalWallRunGate
  (Utilities|FlowControl|Gate true) ; enters at Open
)

(event Custom|CloseWallRunGate
  (Utilities|FlowControl|Gate true) ; enters at Close
)

(event Custom|OpenWallRunGate
  (Utilities|FlowControl|Gate true) ; enters at Open
)

(event Custom|MantleStart
  (bind _changed (CallFunction|SetParkourType "NewEnumerator5"))
  (if _changed
    (CallFunction|PlayCameraShake (select (Utilities|QuickMantle) "/Game/Blueprints/Components/CameraShakes/QuickMantle.QuickMantle_C" "/Game/Blueprints/Components/CameraShakes/Mantle.Mantle_C"))
    (CallFunction|CloseMantleGateCheck)
    (CallFunction|OpenMantleGate)))

(event Custom|CloseMantleGate
  (Utilities|FlowControl|Gate true) ; enters at Close
)

(event Custom|OpenMantleGateCheck
  (Utilities|FlowControl|Gate true) ; enters at Open
)

(event Custom|CloseMantleGateCheck
  (Utilities|FlowControl|Gate true) ; enters at Close
)

(event Custom|OpenMantleGate
  (Utilities|FlowControl|Gate true) ; enters at Open
)

(event Custom|MantleCheck
  (if (Utilities|CanMantle)
    (CallFunction|MantleStart)))

(event Custom|CloseSprintGate
  (Utilities|FlowControl|Gate true) ; enters at Close
)

(event Custom|OpenSprintGate
  (Utilities|FlowControl|Gate true) ; enters at Open
)