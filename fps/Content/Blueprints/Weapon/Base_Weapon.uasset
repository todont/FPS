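; Base weapon Blueprint that loads its stats from a DTWeapon row in the construction script, though the Accuracy assignment is left unconnected.
; StartFire handles Auto mode with a gate and retriggerable-delay loop that spawns projectiles and spends ammo, while StopFire toggles the gate.
; Shots leave the muzzle toward a camera line-trace target, with random Accuracy-based rotation spread.
; Weapon_drop calls a pistol swap when CanFire is false and ammo is empty.
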(event Custom|StopFire
  (Utilities|FlowControl|Gate true) ; enters at Toggle
)

(event Custom|FirePress
  (CallFunction|StartFire))

(event Custom|StartFire
  (switch Utilities|FlowControl|Switch|SwitchonFireMode (Variables|Default|GetFireMode)
    (:NewEnumerator2
      (Utilities|FlowControl|Sequence
        (:then_0
          (goto _label Open))
        (:then_1
          (Utilities|FlowControl|Gate true :!label _label
            (:Exit
              (Utilities|FlowControl|Sequence
                (:then_0
                  (Utilities|FlowControl|RetriggerableDelay (Variables|Default|GetFireRate))
                  (goto _label))
                (:then_1
                  (if (> (Utilities|Struct|BreakWeaponData (Variables|Default|GetWeaponData)) 0)
                    (CallFunction|SpawnProjectile)
                    (Development|PrintString "FIRE" false false)
                    (Variables|Default|SetWeaponData (Utilities|Struct|MakeWeaponData (.MuzzleName (Utilities|Struct|BreakWeaponData (Variables|Default|GetWeaponData))) (.FireMode (Utilities|Struct|BreakWeaponData (Variables|Default|GetWeaponData))) (.FireRate (Utilities|Struct|BreakWeaponData (Variables|Default|GetWeaponData))) (.ReloadDelay (Utilities|Struct|BreakWeaponData (Variables|Default|GetWeaponData))) (.Accuracy (Utilities|Struct|BreakWeaponData (Variables|Default|GetWeaponData))) (.MinDamage (Utilities|Struct|BreakWeaponData (Variables|Default|GetWeaponData))) (.MaxDamage (Utilities|Struct|BreakWeaponData (Variables|Default|GetWeaponData))) (.AmmoMax (Utilities|Struct|BreakWeaponData (Variables|Default|GetWeaponData))) (.Ammo (Utilities|Struct|BreakWeaponData (Variables|Default|GetWeaponData))) (- (.CurrentAmmo (Utilities|Struct|BreakWeaponData (Variables|Default|GetWeaponData))) 1) (.FireAnim (Utilities|Struct|BreakWeaponData (Variables|Default|GetWeaponData))) (.ReloadAnim (Utilities|Struct|BreakWeaponData (Variables|Default|GetWeaponData)))))
                    (Development|PrintString (Utilities|String|ToString(Integer) (- (.CurrentAmmo (Utilities|Struct|BreakWeaponData (Variables|Default|GetWeaponData))) 1)))))))))))))

(event Custom|Weapon_drop
  (if (not (Variables|Default|GetCanFire))
    (if (== (Utilities|Struct|BreakWeaponData (Variables|Default|GetWeaponData)) 0)
      (Development|PrintString "outofammo" true true "(R=1.000000,G=0.052632,B=0.000000,A=1.000000)")
      (CallFunction|SwaptoPistol))))

(event Custom|Release
  (CallFunction|StopFire))

(event Custom|Swap_to_pistol)

(event EventBeginPlay
  (Utilities|FlowControl|Delay 0.2)
  (Development|PrintString (Utilities|String|ToString(Name) (Variables|Default|GetMuzzleName))))

(fn ConstructionScript
  (bind _returnvalue (Utilities|GetDataTableRow "/Game/Blueprints/Weapon/DTWeapon.DTWeapon" (Variables|Default|GetWeapon_Row_Name))
    (:then
      (bind _output_get (Variables|Default|SetWeaponData _returnvalue))
      (Variables|Default|SetMuzzleName (.MuzzleName (Utilities|Struct|BreakWeaponData _output_get)))
      (Variables|Default|SetFireMode (.FireMode (Utilities|Struct|BreakWeaponData _output_get)))
      (Variables|Default|SetFireRate (.FireRate (Utilities|Struct|BreakWeaponData _output_get)))
      (Variables|Default|SetReloadDelay (.ReloadDelay (Utilities|Struct|BreakWeaponData _output_get))))))

(fn CalculateDirection
  (bind _returnvalue (Utilities|MuzzlePosition))
  (bind _character (Variables|Default|GetCharacter))
  (bind _firstpersoncamera (Variables|/Game/Blueprints/FirstPersonBP/FirstPersonCharacter.FirstPersonCharacter_C|GetFirstPersonCamera _character))
  (bind _returnvalue_2 (Transformation|GetWorldTransform _firstpersoncamera))
  (bind _returnvalue_3 (|EndPoint (.rotation _returnvalue_2) (.location _returnvalue_2)))
  (bind (_outhit _returnvalue_4) (Collision|LineTraceForObjects (|Startpoint (.rotation _returnvalue_2) (.location _returnvalue_2)) _returnvalue_3 (Utilities|Array|MakeArray "ObjectTypeQuery1") false 0 "None"))
  (return _returnvalue (Math|Rotator|FindLookatRotation _returnvalue (Math|Vector|SelectVector (.ImpactPoint (Collision|BreakHitResult _outhit)) _returnvalue_3 _returnvalue_4))))

(fn SpawnProjectile
  (Animation|Montage|MontagePlay (Components|SkeletalMesh|GetAnimInstance (Variables|Default|GetWeapon_Mesh)) "/Game/Anims/Weapon/Rifle_Shoot_Montage.Rifle_Shoot_Montage" 1.0 "MontageLength" 0.0 true)
  (bind (_location _rotation) (CallFunction|CalculateDirection))
  (bind _transform (CallFunction|CalculateFinalDirection _location _rotation))
  (Game|SpawnActorfromClass "/Game/Blueprints/Weapon/BP-RifleProj.BP-RifleProj_C" _transform "Undefined" 0 0))

(fn CalculateFinalDirection
  (params (Location :type Vector) (Rotation :type Rotator))
  (bind _accuracy (Variables|Default|GetAccuracy))
  (bind _returnvalue (* _accuracy -1.0))
  (return (Math|Transform|MakeTransform Location (Math|Rotator|CombineRotators Rotation (Math|Rotator|MakeRotator (Math|Random|RandomFloatinRange _returnvalue 0.0) (Math|Random|RandomFloatinRange _returnvalue 0.0) (Math|Random|RandomFloatinRange _returnvalue 0.0))))))